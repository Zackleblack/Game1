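; Stealth-game enemy AI that patrols target points or random locations, investigates noises and chases the player on sight.
; PawnSensing and AIPerception events set sight and hearing flags, which Tick uses to choose between AI MoveTo behaviours.
; Sightings trigger an alert sound and exclamation mark, reset by a retriggerable cooldown.
; Montage-notify sphere-trace hits reload the player's game state, while overlapping the catch box shows a caught widget and teleports the player back.
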(event OnSeePawn(PawnSensing)
  (params (Pawn :type Pawn%20Object%20Reference))
  ;[0.02272 0.05454 0.15 0.5] Pawn See Sensor
  (Utilities|Casting|CastToBP_ThirdPersonCharacterCustom Pawn
    (:then
      (Development|PrintString "I can see you")
      (Variables|Default|SetbPlayerVisible true)
      ;;[0.15 0 0 0] Activate Alert Script
      (Utilities|FlowControl|Sequence
        (:then_0
          (CallFunction|AlertSound))
        (:then_1
          (CallFunction|ChasePlayer))))
    (:CastFailed
      (Development|PrintString "Where did you go?")
      (Utilities|FlowControl|Delay 2.0)
      ;;[0.0462 0.15 0.05304 0] Resume Patrol
      (Variables|Default|SetbPlayerVisible false)
      (CallFunction|PatrolRandom))))

(event OnComponentBeginOverlap(Box)
  (params (OverlappedComponent :type Primitive%20Component%20Object%20Reference) (OtherActor :type Actor%20Object%20Reference) (OtherComp :type Primitive%20Component%20Object%20Reference) (OtherBodyIndex :type Integer) (bFromSweep :type Boolean) (SweepResult :type Hit%20Result%20Structure%20%28by%20ref%29))
  ;[0.15 0.15 0.15 0.5] Caught Box (Component)
  (bind _asbp_third_person_character_custom (Utilities|Casting|CastToBP_ThirdPersonCharacterCustom OtherActor))
  (Components|Movement|StopMovementImmediately (Variables|Character|GetCharacterMovement))
  (Input|DisableInput _asbp_third_person_character_custom 0)
  (Development|PrintString "Haha! Got you!")
  (Utilities|FlowControl|Sequence
    (:then_0
      (Components|Movement|StopMovementImmediately (Variables|Character|GetCharacterMovement))
      (Utilities|FlowControl|RetriggerableDelay 3.0)
      (Variables|Default|SetbCanMove true)
      (CallFunction|PatrolRandom))
    (:then_1
      (bind _returnvalue (UserInterface|CreateWidget "/Game/StealthGame/Core/W_Caught.W_Caught_C"))
      (Utilities|FlowControl|Delay 1.0)
      (UserInterface|Viewport|AddtoViewport _returnvalue 0)
      (Utilities|FlowControl|Sequence
        (:then_0
          (Utilities|FlowControl|Delay 1.0)
          (Transformation|SetActorLocationAndRotation _asbp_third_person_character_custom "1006.615426,3793.547087,77.119232")
          (Development|PrintString "Go back to where you belong (teleport back)")
          (Input|EnableInput _asbp_third_person_character_custom 0))
        (:then_1
          (Utilities|FlowControl|Delay 4.3)
          (Widget|RemovefromParent _returnvalue))))))

(event OnHearNoise(PawnSensing)
  (params (Instigator :type Pawn%20Object%20Reference) (Location :type Vector%20%28by%20ref%29 :default "0, 0, 0") (Volume :type Float%20%28single-precision%29))
  ;[0.15 0.15 0.15 0.5] Hear Noise (PawnSensing)
  (Variables|Default|SetbDidIHearSomething? true)
  (Development|PrintString "I Heard Something")
  (CallFunction|WalkSpeed (Variables|Default|GetSprint%20Speed))
  (Variables|Default|SetbCanMove false)
  (AI|AIMoveTo self Location Instigator 8e+01 false
    (:OnSuccess
      (Utilities|FlowControl|Sequence
        (:then_0
          (Utilities|FlowControl|Delay 6.0)
          (Development|PrintString "Must've been nothing")
          (Utilities|FlowControl|Delay 6.0 :!label _label)
          (Variables|Default|SetbCanMove true)
          (Variables|Default|SetbDidIHearSomething? false)
          (CallFunction|PatrolRandom))
        (:then_1
          (Development|PrintString "I reached Sound"))))
    (:OnFail
      (Development|PrintString "Couldn't reach sound")
      (goto _label))))

(event OnTargetPerceptionUpdated(AIPerception)
  (params (Actor :type Actor%20Object%20Reference) (Stimulus :type AI%20Stimulus%20Structure))
  ;[0.15 0.15 0.15 0.5] Caught Box (Component)
  ;;[0.03515 0.03659 0.15 0.5] Searching Voice Sound
  (Variables|Default|SetbDidIHearSomething? (.bsuccessfullysensed Stimulus))
  (AI|AIMoveTo self (.stimuluslocation Stimulus) 0 5.0 false
    (:OnSuccess
      (Development|PrintString "Reached Sound Location")
      (Utilities|FlowControl|Delay 5.0)
      (Variables|Default|SetbCanMove true)
      (Variables|Default|SetbDidIHearSomething? false)
      (CallFunction|PatrolRandom))))

(event Custom|Chase%20Player
  ;[0.4087 0 0 0.5] Chase Player
  (Utilities|FlowControl|Delay 0.4)
  (CallFunction|WalkSpeed (Variables|Default|GetSprint%20Speed))
  (Variables|Default|SetbCanMove true)
  (AI|AIMoveTo self "0, 0, 0" (Game|GetPlayerCharacter 0) 8e+01 false
    (:OnSuccess
      (CallFunction|Attack)
      (Utilities|FlowControl|Delay 5.0)
      (CallFunction|ResetAttack))))

(event Custom|Alert%20Sound
  (bind _exclamation_mark_a4122072 (Variables|Default|GetExclamation_Mark_A4122072))
  ;[0.15 0.01797 0.01797 0.5] Alert Script
  (if (Variables|Default|GetbDidAlertGoOff?) ; T/F Did you get alerted?
    (CallFunction|AlertCooldown) ; Play this if Alert Went off
    (else
      (Variables|Default|SetbDidAlertGoOff? true) ; Set on to activate alert
      (Audio|PlaySoundatLocation "/Game/Alert_cue.Alert_cue" (.location (Transformation|GetActorTransform)) "0, 0, 0" 1.0 1.0 0.0 0 0 0 0) ; When Spotted, play sound
      (Development|SetHiddeninGame _exclamation_mark_a4122072 false false) ; Show Exclamation Mark
      (Utilities|FlowControl|Delay 2.0) ; Wait 2 seconds
      (Development|SetHiddeninGame _exclamation_mark_a4122072 true false) ; Put Exclamation Mark back to hidden
    )))

(event Custom|Patrol%20Random
  ;[0.07147 0.15 0.06058 0.5] Patrol Random
  (CallFunction|WalkSpeed (Variables|Default|GetWalk%20Speed))
  (Variables|Default|SetbCanMove false)
  (AI|AIMoveTo self (.RandomLocation (AI|Navigation|GetRandomReachablePointinRadius (Transformation|GetActorLocation) 3e+03 0 0)) 0 8e+01 false
    (:OnSuccess
      (Utilities|FlowControl|Delay 6.0)
      (Variables|Default|SetbCanMove true)
      (CallFunction|PatrolRandom))))

(event Custom|Attack
  (bind _mesh (Variables|Character|GetMesh))
  (bind _returnvalue (Transformation|GetSocketLocation _mesh "hand_r"))
  ;[0.15 0.1407 0.04319 0.5] Bonk
  (Utilities|FlowControl|DoOnce false ; Only Reset Attack on miss.
    (:Completed
      (bind _notifyname (Animation|Montage|PlayMontage (Variables|Character|GetMesh) "/Game/StealthGame/Characters/Enemies/AM_Attack_01.AM_Attack_01") ; Play the AM_Attack_01
        (:OnCompleted
          (if (Variables|Default|GetbHostile) ; Keep attacking if you haven't landed the hit.
            (CallFunction|ResetAttack)))
        (:OnNotifyBegin
          (switch name _notifyname ; Pick the proper attack type(standard when there is more than one type of attack)
            (:AttackDamage
              (Development|PrintString "I'm attacking!")
              (bind (_outhits _returnvalue_2) (Collision|MultiSphereTraceForObjects _returnvalue (+ _returnvalue (* (Transformation|GetActorForwardVector) (Variables|Default|GetMelee%20Trace%20Distance))) (Variables|Default|GetMelee%20Trace%20Radius) (Utilities|Array|MakeArray "ObjectTypeQuery3") false 0 "None")) ; Trace forward from hand socket.
              (if _returnvalue_2 ; If a pawn is hit in that trace...
                (for _array_element _outhits ; ...loop through the results....
                  (bind _asbp_third_person_character_custom (Utilities|Casting|CastToBP_ThirdPersonCharacterCustom (.HitActor (Collision|BreakHitResult _array_element))))
                  (Default|LoadGameState _asbp_third_person_character_custom)
                  (Development|PrintString "Game Over"))))))))))

(event Custom|MoveToNextPatrolPoint
  ;[0.15 0.15 0.15 0.5] Move to Patrol Point
  (CallFunction|WalkSpeed (Variables|Default|GetWalk%20Speed))
  (Variables|Default|SetbCanMove true)
  (AI|AIMoveTo self "0, 0, 0" (Utilities|Array|Get(acopy) (Variables|Default|GetPatrolTargetPoints) (Variables|Default|GetPatrolTargetPointINdex)) 5e+01 false
    (:OnSuccess
      (Utilities|FlowControl|Delay 6.0)
      (Variables|Default|SetbCanMove true)
      (CallFunction|SetNextPatrolPointIndex))))

(event Custom|ResetAttack
  (bind _mesh (Variables|Character|GetMesh))
  (bind _returnvalue (Transformation|GetSocketLocation _mesh "hand_r"))
  ;[0.15 0.1407 0.04319 0.5] Bonk
  (Utilities|FlowControl|DoOnce false) ; enters at Reset
)

(event Custom|Alert%20Cooldown
  ;[0.15 0.15 0.15 0.5] Alert Cooldown
  (Utilities|FlowControl|RetriggerableDelay 5.0) ; Keeps playing till you've been outta sight\nFor longer then 5 seconds
  (Development|PrintString "Where did you go?")
  (Variables|Default|SetbDidAlertGoOff? false) ; Reset Alert Script
  (Variables|Default|SetbPlayerVisible false) ; Hide the player
  (CallFunction|PatrolRandom) ; Resume patrol
)

(event Custom|Set%20Next%20Patrol%20Point%20Index
  ;[0.04888 0.15 0.03464 0.5] Patrol Array Index
  (Variables|Default|SetPatrolTargetPointINdex (Math|Integer|%(Integer) (+ (Variables|Default|GetPatrolTargetPointINdex) 1) (Utilities|Array|Length (Variables|Default|GetPatrolTargetPoints)))))

(event Custom|Noise%20Heard
  ;[0.6609 0.15 0.15 0.7913] Noise Focus Delay
  (Utilities|FlowControl|Delay 8.0)
  (Variables|Default|SetbDidIHearSomething? false))

(event Custom|You've%20Been%20Caught
  (Components|Movement|StopMovementImmediately (Variables|Character|GetCharacterMovement))
  (Utilities|FlowControl|Delay 2.0)
  (CallFunction|PatrolRandom))

(event Custom|EnemySpawned
  (CallFunction|PatrolRandom))

(event EventBeginPlay
  ;[0.15 0.15 0.15 0.5] Event Begin Play
  (if (Variables|Default|GetbTargetPointMovement)
    (CallFunction|MovetoNextPatrolPoint)
    (else
      (CallFunction|PatrolRandom))))

(event EventTick
  (params (DeltaSeconds :type Float%20%28single-precision%29))
  (bind _bplayervisible (Variables|Default|GetbPlayerVisible))
  ;[0.15 0.03975 0.03724 0.5] Hierarchy Branch (Tick)
  (Variables|Default|SetbDidISpawn? true)
  (if (Variables|Default|GetbDidIHearSomething?)
    (CallFunction|NoiseHeard)
    (elif (Variables|Default|GetbCanMove)
      (if _bplayervisible
        (CallFunction|ChasePlayer)
        (elif (Variables|Default|GetbTargetPointMovement)
          (CallFunction|MovetoNextPatrolPoint)
          (else
            (CallFunction|PatrolRandom))))
      (elif _bplayervisible
        (CallFunction|ChasePlayer)))))

(fn ConstructionScript)

(fn WalkSpeed
  (params (New%20Walk%20Speed :type Float%20%28double-precision%29))
  (Variables|/Script/Engine.CharacterMovementComponent|SetMaxWalkSpeed (Variables|Character|GetCharacterMovement) New%20Walk%20Speed))

(fn StartedSprint
  (Variables|Default|SetMax%20Speed 0.0))