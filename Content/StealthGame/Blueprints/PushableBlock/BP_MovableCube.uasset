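; BP_MovableCube is a pushable block for the stealth game that moves only while the player character is in contact with its trigger areas.
; Two collision components, one per X and Y axis, toggle physics simulation on PushableBox as BP_ThirdPersonCharacterCustom begins or ends overlap.
; The same overlap events set the character's IsPushing flag.
; Each trigger acts independently, so leaving either one switches off physics and pushing.
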(event OnComponentBeginOverlap(YAxisCollision)
  (params (OverlappedComponent :type Primitive%20Component%20Object%20Reference) (OtherActor :type Actor%20Object%20Reference) (OtherComp :type Primitive%20Component%20Object%20Reference) (OtherBodyIndex :type Integer) (bFromSweep :type Boolean) (SweepResult :type Hit%20Result%20Structure%20%28by%20ref%29))
  ;[0.15 0.15 0.15 0.5] Y Axis Collision
  (bind _asbp_third_person_character_custom (Utilities|Casting|CastToBP_ThirdPersonCharacterCustom OtherActor))
  (Physics|SetSimulatePhysics (Variables|Default|GetPushableBox) true)
  (Variables|/Game/StealthGame/Core/Characters/PlayerCharacter/BP_ThirdPersonCharacterCustom.BP_ThirdPersonCharacterCustom_C|SetbIsPushing _asbp_third_person_character_custom true))

(event OnComponentEndOverlap(YAxisCollision)
  (params (OverlappedComponent :type Primitive%20Component%20Object%20Reference) (OtherActor :type Actor%20Object%20Reference) (OtherComp :type Primitive%20Component%20Object%20Reference) (OtherBodyIndex :type Integer))
  ;[0.15 0.15 0.15 0.5] Y Axis Collision
  (bind _asbp_third_person_character_custom (Utilities|Casting|CastToBP_ThirdPersonCharacterCustom OtherActor))
  (Physics|SetSimulatePhysics (Variables|Default|GetPushableBox) false)
  (Variables|/Game/StealthGame/Core/Characters/PlayerCharacter/BP_ThirdPersonCharacterCustom.BP_ThirdPersonCharacterCustom_C|SetbIsPushing _asbp_third_person_character_custom false))

(event OnComponentBeginOverlap(XAxisCollision1)
  (params (OverlappedComponent :type Primitive%20Component%20Object%20Reference) (OtherActor :type Actor%20Object%20Reference) (OtherComp :type Primitive%20Component%20Object%20Reference) (OtherBodyIndex :type Integer) (bFromSweep :type Boolean) (SweepResult :type Hit%20Result%20Structure%20%28by%20ref%29))
  ;[0.15 0.15 0.15 0.5] X Axis Collision
  (bind _asbp_third_person_character_custom (Utilities|Casting|CastToBP_ThirdPersonCharacterCustom OtherActor))
  (Physics|SetSimulatePhysics (Variables|Default|GetPushableBox) true)
  (Variables|/Game/StealthGame/Core/Characters/PlayerCharacter/BP_ThirdPersonCharacterCustom.BP_ThirdPersonCharacterCustom_C|SetbIsPushing _asbp_third_person_character_custom true))

(event OnComponentEndOverlap(XAxisCollision1)
  (params (OverlappedComponent :type Primitive%20Component%20Object%20Reference) (OtherActor :type Actor%20Object%20Reference) (OtherComp :type Primitive%20Component%20Object%20Reference) (OtherBodyIndex :type Integer))
  ;[0.15 0.15 0.15 0.5] X Axis Collision
  (bind _asbp_third_person_character_custom (Utilities|Casting|CastToBP_ThirdPersonCharacterCustom OtherActor))
  (Physics|SetSimulatePhysics (Variables|Default|GetPushableBox) false)
  (Variables|/Game/StealthGame/Core/Characters/PlayerCharacter/BP_ThirdPersonCharacterCustom.BP_ThirdPersonCharacterCustom_C|SetbIsPushing _asbp_third_person_character_custom false))

(fn ConstructionScript)