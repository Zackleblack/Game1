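; BP_BookshelfPuzzle is a bookshelf puzzle that removes a glass component once the player places a collected book.
; PickUpBook sets a HasBook flag, which gates the Interact event.
; A successful Interact unhides the book's static mesh, marks the shelf complete and calls DestroyGlass, which destroys the Glass component.
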(event Custom|Destroy%20Glass
  (if (Variables|Default|GetbShelfIsComplete)
    (Components|DestroyComponent (Variables|Default|GetGlass))))

(event EventInteract
  (if (Variables|Default|GetbHasBook?)
    (Development|SetHiddeninGame (Variables|Default|GetStaticMesh) false false)
    (Variables|Default|SetbShelfIsComplete true)
    (CallFunction|DestroyGlass)))

(event EventPickUpBook
  (Variables|Default|SetbHasBook? true))

(fn ConstructionScript)