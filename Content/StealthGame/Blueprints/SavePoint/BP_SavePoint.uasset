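; BP_SavePoint is a rotating save point that saves game state when BP_ThirdPersonCharacterCustom overlaps its collision.
; The overlap calls the character's SaveGameState and temporarily speeds up RotatingMovement.
; A parallel Sequence branch, not gated by the character cast, plays a shutter sound and shows the W_GameSaved widget briefly.
; The character leaving the collision also triggers a delayed removal of that widget.
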(event OnComponentBeginOverlap(Collision)
  (params (OverlappedComponent :type Primitive%20Component%20Object%20Reference) (OtherActor :type Actor%20Object%20Reference) (OtherComp :type Primitive%20Component%20Object%20Reference) (OtherBodyIndex :type Integer) (bFromSweep :type Boolean) (SweepResult :type Hit%20Result%20Structure%20%28by%20ref%29))
  (bind _rotatingmovement (Variables|Default|GetRotatingMovement))
  (if true
    (Utilities|FlowControl|Sequence
      (:then_0
        (bind _asbp_third_person_character_custom (Utilities|Casting|CastToBP_ThirdPersonCharacterCustom OtherActor))
        (Default|SaveGameState _asbp_third_person_character_custom)
        (Variables|/Script/Engine.RotatingMovementComponent|SetRotationRate _rotatingmovement "0.000000,360.000000,0.000000")
        (Utilities|FlowControl|Delay 5.0)
        (Variables|/Script/Engine.RotatingMovementComponent|SetRotationRate _rotatingmovement "0.000000,180.000000,0.000000"))
      (:then_1
        (Audio|PlaySound2D "/Engine/VREditor/Sounds/UI/Camera_Shutter.Camera_Shutter" 1.0 1.0 0.0 0 0)
        (bind _returnvalue (UserInterface|CreateWidget "/Game/StealthGame/Core/W_GameSaved.W_GameSaved_C"))
        (UserInterface|Viewport|AddtoViewport _returnvalue 0)
        (Utilities|FlowControl|Delay 4.0)
        (Widget|RemovefromParent _returnvalue)))))

(event OnComponentEndOverlap(Collision)
  (params (OverlappedComponent :type Primitive%20Component%20Object%20Reference) (OtherActor :type Actor%20Object%20Reference) (OtherComp :type Primitive%20Component%20Object%20Reference) (OtherBodyIndex :type Integer))
  (Utilities|Casting|CastToBP_ThirdPersonCharacterCustom OtherActor)
  (Utilities|FlowControl|Delay 4.0)
  (Widget|RemovefromParent (stale OnComponentBeginOverlap(Collision) _returnvalue)))

(fn ConstructionScript)