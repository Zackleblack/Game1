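; Enemy wave manager for the stealth game that respawns enemies once the level is cleared.
; NewEnemyWaveCHeck counts BP_Enemy actors and, when none remain, starts SpawnNewEnemies and spawns a BP_Key at the supplied transform.
; SpawnNewEnemies waits briefly, then calls SpawnNewEnemy on every BP_EnemySpawner found through GetAllActorsOfClass.
; On-screen debug prints report the spawner count at BeginPlay and wave progress, using random colors for each spawner.
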(event Custom|NewEnemyWaveCHeck
  (params (Transform :type Transform))
  (Development|PrintString "Checking enemy count")
  (bind _outactors (Actor|GetAllActorsOfClass "/Game/Blueprints/BP_Enemy.BP_Enemy_C"))
  (if (> (Utilities|Array|Length _outactors) 0) ; If all enemies in level are\nGreater than zero, do nothing
    (Development|PrintString "There are still monsters")
    (else
      (CallFunction|SpawnNewEnemies)
      (Game|SpawnActorfromClass "/Game/Blueprints/BP_Key.BP_Key_C" Transform "AlwaysSpawn" "MultiplyWithRoot" 0 0))))

(event Custom|Spawn%20New%20Enemies
  (Development|PrintString "spawning new enemies in 4 seconds" true true "(R=1.000000,G=0.000000,B=0.188499,A=1.000000)" 5.0)
  (Utilities|FlowControl|Delay 4.0)
  (bind _outactors (Actor|GetAllActorsOfClass "/Game/Blueprints/BP_EnemySpawner.BP_EnemySpawner_C"))
  (for (_array_element _array_index) _outactors ; the Array element is a reference\nto each spawner in the array
    (Default|SpawnNewEnemy _array_element)
    ;[0.15 0.15 0.15 0.5] Use the Print String, Append Node
    ; Array Index, and the GetDisplayName
    ; node to print string for each spawner
    (Development|PrintString (Utilities|String|Append (Utilities|String|ToString(Integer) _array_index) ". " (Utilities|GetDisplayName _array_element) "Is spawning...") true true (Utilities|Struct|MakeLinearColor (Math|Random|RandomFloat) (Math|Random|RandomFloat) (Math|Random|RandomFloat) 1.0) 5.0) ; Drag backwards from\nIn String to get to Append
  )
  (Development|PrintString "New Wave Complete!"))

(event EventBeginPlay
  (Development|PrintString "Spawn Manager is active")
  (bind _outactors (Actor|GetAllActorsOfClass "/Game/Blueprints/BP_EnemySpawner.BP_EnemySpawner_C")) ; Find all the spawners in level
  (Development|PrintString (Utilities|String|Append "There are" (Utilities|String|ToString(Integer) (Utilities|Array|Length _outactors)) "Spawners in the level" "There are " "##" "Enemies in the level") true true "(R=0.385304,G=1.000000,B=0.000000,A=1.000000)" 1e+01))

(fn ConstructionScript)