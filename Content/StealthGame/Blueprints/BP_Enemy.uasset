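; BP_Enemy is a stealth-game enemy that dies when BP_ThirdPersonCharacter overlaps its capsule.
; The overlap prints a debug message and plays a hit sound while a one-second delay runs before destruction.
; It caches its transform, destroys itself, then finds BP_EnemySpawnManager by class and passes that transform to its wave check.
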(event OnComponentBeginOverlap(Capsule)
  (params (OverlappedComponent :type Primitive%20Component%20Object%20Reference) (OtherActor :type Actor%20Object%20Reference) (OtherComp :type Primitive%20Component%20Object%20Reference) (OtherBodyIndex :type Integer) (bFromSweep :type Boolean) (SweepResult :type Hit%20Result%20Structure%20%28by%20ref%29))
  (Utilities|Casting|CastToBP_ThirdPersonCharacter OtherActor) ; Was it the player that ran into us?
  (Utilities|FlowControl|Sequence
    (:then_0
      (Development|PrintString "Dies cutely")
      (Utilities|FlowControl|Delay 1.0) ; Process the death
      (Variables|Default|SetTransform%20At%20Death (Transformation|GetWorldTransform (Variables|Default|GetDefaultSceneRoot)))
      (Actor|DestroyActor) ; Dies
      ;[0.3853 1 0] Tell the manager that we are dying
      (bind _returnvalue (Actor|GetActorOfClass "/Game/Blueprints/BP_EnemySpawnManager.BP_EnemySpawnManager_C")) ; Find the enemy spawn manager
      (Default|NewEnemyWaveCHeck _returnvalue (Variables|Default|GetTransform%20At%20Death)) ; ask the enemy spawn manager to\ncheck how many enemies are left.
    )
    (:then_1
      (Audio|PlaySound2D "/Game/StarterContent/Audio/Hit_Sound.Hit_Sound" 1.0 1.0 0.0 0 0))))

(fn ConstructionScript)