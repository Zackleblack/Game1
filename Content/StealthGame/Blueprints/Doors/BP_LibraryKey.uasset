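; BP_LibraryKey is a key pickup in the stealth game that reports to a referenced Door when collected.
; A Box overlap by the custom third-person character sets NearKey and shows the W_Pickup widget; leaving removes the widget but leaves NearKey set.
; Interact calls the Door's PickUpKeyMessage, plays a pickup sound, destroys the key and then sets KeyWasGot.
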(event OnComponentBeginOverlap(Box)
  (params (OverlappedComponent :type Primitive%20Component%20Object%20Reference) (OtherActor :type Actor%20Object%20Reference) (OtherComp :type Primitive%20Component%20Object%20Reference) (OtherBodyIndex :type Integer) (bFromSweep :type Boolean) (SweepResult :type Hit%20Result%20Structure%20%28by%20ref%29))
  (Utilities|Casting|CastToBP_ThirdPersonCharacterCustom OtherActor)
  (Variables|Default|SetbNearKey? true)
  (bind _returnvalue (UserInterface|CreateWidget "/Game/StealthGame/Blueprints/Doors/W_Pickup.W_Pickup_C"))
  (UserInterface|Viewport|AddtoViewport _returnvalue 0))

(event OnComponentEndOverlap(Box)
  (params (OverlappedComponent :type Primitive%20Component%20Object%20Reference) (OtherActor :type Actor%20Object%20Reference) (OtherComp :type Primitive%20Component%20Object%20Reference) (OtherBodyIndex :type Integer))
  (Utilities|Casting|CastToBP_ThirdPersonCharacterCustom OtherActor)
  (Widget|RemovefromParent (stale OnComponentBeginOverlap(Box) _returnvalue)))

(event EventInteract
  (Class|BPIDoor|PickUpKey(Message) (Variables|Default|GetDoor))
  (Audio|PlaySound2D "/Game/StealthGame/Blueprints/Doors/KeyPickup_Cue.KeyPickup_Cue" 1.0 1.0 0.0 0 0)
  (Actor|DestroyActor)
  (Variables|Default|SetbKeyWasGot true))

(fn ConstructionScript)