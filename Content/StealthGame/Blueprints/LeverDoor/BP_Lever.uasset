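; BP_Lever is an interactable lever that signals a referenced door when used.
; Its Interact event sends InteractWithObjectMessage to DoorReference, then starts the lever animation and the indicator light change.
; A timeline lerps the static mesh's pitch to swing the lever, while the light switches to a green material after a short delay.
; A PickUpKeyMessage call to the door is present but never runs.
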(event Custom|Lever%20Positon%20Change
  (bind _swap_on (Timeline|Timeline Play)
    (:Update
      (Transformation|SetRelativeRotation (Variables|Default|GetStaticMesh) (Math|Rotator|MakeRotator 0.0 (Math|Float|Lerp -4e+01 -1.4e+02 _swap_on) 0.0) false false))))

(event Custom|Light%20Change
  (Utilities|FlowControl|Delay 3.0)
  (Rendering|Material|SetMaterial (Variables|Default|GetLight) 0 "/Game/StealthGame/Blueprints/BookPuzzle/Materials/MI_GreenBookPuzzle.MI_GreenBookPuzzle"))

(event EventInteract
  (Class|BPIInteractObject|InteractwithObject(Message) (Variables|Default|GetDoor%20Reference))
  (Utilities|FlowControl|Sequence
    (:then_0
      (CallFunction|LeverPositonChange))
    (:then_1
      (CallFunction|LightChange))))

(fn ConstructionScript)