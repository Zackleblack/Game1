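; Falling platform actor for the stealth game that drops after the third-person character steps on it, then returns to its start.
; On overlap while ready, it waits a delay, enables physics simulation to fall, then after a fall duration disables physics.
; A timeline lerps it back to the transform captured at BeginPlay and re-arms it.
; Material swaps and debug prints mark each state.
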(event Custom|Activate
  (Variables|Default|SetisReady false)
  (Development|PrintString "Starting Countdown")
  (Rendering|Material|SetMaterial (Variables|Default|GetPlatform) 0 "/Game/Materials/FallingPlatforms/MI_ActivePlatform.MI_ActivePlatform")
  (Utilities|FlowControl|Delay (Variables|PlatformSettings|GetFallDelayDuration))
  (CallFunction|Fall))

(event Custom|Fall
  (Development|PrintString "Im falling")
  (Rendering|Material|SetMaterial (Variables|Default|GetPlatform) 0 "/Game/Materials/FallingPlatforms/MI_FallingPlatform.MI_FallingPlatform")
  (Physics|SetSimulatePhysics (Variables|Default|GetPlatform) true)
  (Utilities|FlowControl|Delay (Variables|Default|GetFall%20Duration))
  (CallFunction|Reset))

(event Custom|Reset
  (Development|PrintString "Reseting Platform")
  (Rendering|Material|SetMaterial (Variables|Default|GetPlatform) 0 "/Game/Materials/FallingPlatforms/MI_ResettingPlatform.MI_ResettingPlatform")
  (Physics|SetSimulatePhysics (Variables|Default|GetPlatform) false)
  (Variables|Default|SetFalling%20Position (Transformation|GetWorldTransform (Variables|Default|GetPlatform)))
  (bind _newtrack_0 (Timeline|GoBackToStartTransform PlayFromStart)
    (:Update
      ;[0.15 0.15 0.15 0.5] Timeline update
      (Transformation|SetWorldTransform (Variables|Default|GetPlatform) (Math|Transform|Lerp(Transform) (Variables|Default|GetFalling%20Position) (Variables|Default|GetStarting%20Transform) _newtrack_0) false false))
    (:Finished
      ;[0.15 0.15 0.15 0.5] Timeline finished
      (Variables|Default|SetisReady true)
      (Rendering|Material|SetMaterial (Variables|Default|GetPlatform) 0 "/Game/StarterContent/Materials/M_Basic_Wall.M_Basic_Wall"))))

(event Collision|EventActorBeginOverlap
  (params (OtherActor :type Actor%20Object%20Reference))
  (Development|PrintString "someone stepped on me")
  (Rendering|Material|SetMaterial (Variables|Default|GetPlatform) 0 "/Game/Materials/FallingPlatforms/MI_ReadyPlatform.MI_ReadyPlatform")
  (if (Variables|Default|GetisReady) ; Is platform ready to fall
    (Utilities|Casting|CastToBP_ThirdPersonCharacter OtherActor)
    (CallFunction|Activate)))

(event EventBeginPlay
  ;[0.15 0.15 0.15 0.5] Event Start
  (Variables|Default|SetStarting%20Transform (Transformation|GetWorldTransform (Variables|Default|GetPlatform))) ; capture starting position
)

(fn ConstructionScript)