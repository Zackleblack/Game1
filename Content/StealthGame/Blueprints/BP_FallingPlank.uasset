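; BP_FallingPlank is a plank in the stealth game, apparently meant to be pushed over by the player, but currently unfinished.
; Its collision box sets IsPlayerOn as BP_ThirdPersonCharacterCustom enters or leaves, with debug prints for any overlapping actor.
; The push logic, which plays the Rotate timeline when IsPlayerOn is true, is disconnected and never runs.
; The Interact event is empty, so interacting does nothing.
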(event OnComponentBeginOverlap(Colision)
  (params (OverlappedComponent :type Primitive%20Component%20Object%20Reference) (OtherActor :type Actor%20Object%20Reference) (OtherComp :type Primitive%20Component%20Object%20Reference) (OtherBodyIndex :type Integer) (bFromSweep :type Boolean) (SweepResult :type Hit%20Result%20Structure%20%28by%20ref%29))
  (Development|PrintString "You are on collision Box")
  (Utilities|Casting|CastToBP_ThirdPersonCharacterCustom OtherActor)
  (Variables|Default|SetbIsPlayerOn? true))

(event OnComponentEndOverlap(Colision)
  (params (OverlappedComponent :type Primitive%20Component%20Object%20Reference) (OtherActor :type Actor%20Object%20Reference) (OtherComp :type Primitive%20Component%20Object%20Reference) (OtherBodyIndex :type Integer))
  (Development|PrintString "You left the collision Box")
  (Utilities|Casting|CastToBP_ThirdPersonCharacterCustom OtherActor)
  (Variables|Default|SetbIsPlayerOn? false))

(event EventBeginPlay)

(event Collision|EventActorBeginOverlap
  (params (OtherActor :type Actor%20Object%20Reference)))

(event EventTick
  (params (DeltaSeconds :type Float%20%28single-precision%29)))

(event EventInteract)

(fn ConstructionScript)