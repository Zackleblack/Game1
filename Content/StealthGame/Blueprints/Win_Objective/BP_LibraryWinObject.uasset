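; BP_LibraryWinObject is the library win objective: a golden book the player picks up to unlock the level's win spots.
; Its Box trigger shows a press-E prompt; Interact sets WinUnlock, notifies the character, plays a sound, destroys the book components and shows book and timed leave widgets.
; Overlapping WinSpot or WinSpot2 calls YourWinner once unlocked.
; Only WinSpot2 shows a need-book widget while locked.
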(event OnComponentBeginOverlap(Box)
  (params (OverlappedComponent :type Primitive%20Component%20Object%20Reference) (OtherActor :type Actor%20Object%20Reference) (OtherComp :type Primitive%20Component%20Object%20Reference) (OtherBodyIndex :type Integer) (bFromSweep :type Boolean) (SweepResult :type Hit%20Result%20Structure%20%28by%20ref%29))
  (Utilities|Casting|CastToBP_ThirdPersonCharacterCustom OtherActor)
  (bind _returnvalue (UserInterface|CreateWidget "/Game/StealthGame/Core/Characters/PlayerCharacter/W_PressE.W_PressE_C"))
  (UserInterface|Viewport|AddtoViewport _returnvalue 0))

(event OnComponentEndOverlap(Box)
  (params (OverlappedComponent :type Primitive%20Component%20Object%20Reference) (OtherActor :type Actor%20Object%20Reference) (OtherComp :type Primitive%20Component%20Object%20Reference) (OtherBodyIndex :type Integer))
  (Utilities|Casting|CastToBP_ThirdPersonCharacterCustom OtherActor)
  (Widget|RemovefromParent (stale OnComponentBeginOverlap(Box) _returnvalue)))

(event OnComponentBeginOverlap(WinSpot)
  (params (OverlappedComponent :type Primitive%20Component%20Object%20Reference) (OtherActor :type Actor%20Object%20Reference) (OtherComp :type Primitive%20Component%20Object%20Reference) (OtherBodyIndex :type Integer) (bFromSweep :type Boolean) (SweepResult :type Hit%20Result%20Structure%20%28by%20ref%29))
  (bind _asbp_third_person_character_custom (Utilities|Casting|CastToBP_ThirdPersonCharacterCustom OtherActor))
  (if (Variables|Default|GetbWinUnlock)
    (Default|YourWinner _asbp_third_person_character_custom)))

(event OnComponentBeginOverlap(WinSpot2)
  (params (OverlappedComponent :type Primitive%20Component%20Object%20Reference) (OtherActor :type Actor%20Object%20Reference) (OtherComp :type Primitive%20Component%20Object%20Reference) (OtherBodyIndex :type Integer) (bFromSweep :type Boolean) (SweepResult :type Hit%20Result%20Structure%20%28by%20ref%29))
  (bind _asbp_third_person_character_custom (Utilities|Casting|CastToBP_ThirdPersonCharacterCustom OtherActor))
  (if (Variables|Default|GetbWinUnlock)
    (Default|YourWinner _asbp_third_person_character_custom)
    (else
      (bind _returnvalue (UserInterface|CreateWidget "/Game/StealthGame/Blueprints/Win_Objective/W_NeedBook.W_NeedBook_C"))
      (UserInterface|Viewport|AddtoViewport _returnvalue 0))))

(event OnComponentEndOverlap(WinSpot2)
  (params (OverlappedComponent :type Primitive%20Component%20Object%20Reference) (OtherActor :type Actor%20Object%20Reference) (OtherComp :type Primitive%20Component%20Object%20Reference) (OtherBodyIndex :type Integer))
  (Utilities|Casting|CastToBP_ThirdPersonCharacterCustom OtherActor)
  (Widget|RemovefromParent (stale OnComponentBeginOverlap(WinSpot2) _returnvalue)))

(event EventBeginPlay
  (Variables|Default|SetbWinUnlock false))

(event EventInteract
  (Variables|Default|SetbWinUnlock true)
  (bind _asbp_third_person_character_custom (Utilities|Casting|CastToBP_ThirdPersonCharacterCustom (Game|GetPlayerCharacter 0)))
  (Default|GoldenBookPickUp _asbp_third_person_character_custom)
  (Audio|PlaySound2D "/Game/StealthGame/Blueprints/Doors/KeyPickup_Cue.KeyPickup_Cue" 1.0 1.0 0.0 0 0)
  (Utilities|FlowControl|Sequence
    (:then_1
      (Components|DestroyComponent (Variables|Default|GetGolden%20Book)))
    (:then_2
      (bind _returnvalue (UserInterface|CreateWidget "/Game/PickupWidget/W_WinningBook.W_WinningBook_C"))
      (UserInterface|Viewport|AddtoViewport _returnvalue 0)
      (Utilities|FlowControl|Delay 0.2)
      (bind _returnvalue_2 (UserInterface|CreateWidget "/Game/WBP_Leave.WBP_Leave_C"))
      (UserInterface|Viewport|AddtoViewport _returnvalue_2 0)
      (Utilities|FlowControl|Delay 5.0)
      (Widget|RemovefromParent _returnvalue_2))))

(fn ConstructionScript)