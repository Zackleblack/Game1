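; BP_MusicZone is a trigger actor that starts and stops a music track as the player passes through it.
; Overlapping MusicStart with a Player-tagged actor spawns the Sound variable as 2D audio, stores it in Music and fades it in.
; Overlapping MusicEnd fades that stored component out if it is valid.
; Each trigger is gated by its own DoOnce with no reset, so it fires only once.
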(event OnComponentBeginOverlap(MusicStart)
  (params (OverlappedComponent :type Primitive%20Component%20Object%20Reference) (OtherActor :type Actor%20Object%20Reference) (OtherComp :type Primitive%20Component%20Object%20Reference) (OtherBodyIndex :type Integer) (bFromSweep :type Boolean) (SweepResult :type Hit%20Result%20Structure%20%28by%20ref%29))
  (if (Actor|ActorHasTag OtherActor "Player")
    (Utilities|FlowControl|DoOnce false
      (:Completed
        (Development|PrintString "Music is playing")
        (bind _returnvalue (Audio|SpawnSound2D (Variables|Default|GetSound) 0.35 1.0 0.0 0))
        (bind _output_get (Variables|Default|SetMusic _returnvalue))
        (Audio|Components|Audio|FadeIn _output_get 0.5 0.35 0.0 "Linear" :!class /Script/Engine.AudioComponent)))))

(event OnComponentBeginOverlap(MusicEnd)
  (params (OverlappedComponent :type Primitive%20Component%20Object%20Reference) (OtherActor :type Actor%20Object%20Reference) (OtherComp :type Primitive%20Component%20Object%20Reference) (OtherBodyIndex :type Integer) (bFromSweep :type Boolean) (SweepResult :type Hit%20Result%20Structure%20%28by%20ref%29))
  (if (Actor|ActorHasTag OtherActor "Player")
    (Utilities|FlowControl|DoOnce false
      (:Completed
        (bind _music (Variables|Default|GetMusic)
          (:then
            (Audio|Components|Audio|FadeOut _music 0.5 0.0 "Linear" :!class /Script/Engine.AudioComponent))
          (:else))))))

(event EventBeginPlay)

(event Collision|EventActorBeginOverlap
  (params (OtherActor :type Actor%20Object%20Reference)))

(event EventTick
  (params (DeltaSeconds :type Float%20%28single-precision%29)))

(fn ConstructionScript)