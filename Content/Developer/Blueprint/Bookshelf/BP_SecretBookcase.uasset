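; BP_SecretBookcase is an interactable secret bookcase that slides aside once when its Interact event fires.
; A DoOnce plays a grab sound and runs a Timeline that nudges the actor along negative X from its current location each update, then flags it as moved.
; A trigger box shows a press-E widget to the custom third-person character until the bookcase has moved, removing it when overlap ends.
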(event OnComponentBeginOverlap(Box)
  (params (OverlappedComponent :type Primitive%20Component%20Object%20Reference) (OtherActor :type Actor%20Object%20Reference) (OtherComp :type Primitive%20Component%20Object%20Reference) (OtherBodyIndex :type Integer) (bFromSweep :type Boolean) (SweepResult :type Hit%20Result%20Structure%20%28by%20ref%29))
  (if (not (Variables|Default|GetbMovedObject?))
    (Utilities|Casting|CastToBP_ThirdPersonCharacterCustom OtherActor)
    (bind _returnvalue (UserInterface|CreateWidget "/Game/StealthGame/Core/Characters/PlayerCharacter/W_PressE.W_PressE_C"))
    (UserInterface|Viewport|AddtoViewport _returnvalue 0)))

(event OnComponentEndOverlap(Box)
  (params (OverlappedComponent :type Primitive%20Component%20Object%20Reference) (OtherActor :type Actor%20Object%20Reference) (OtherComp :type Primitive%20Component%20Object%20Reference) (OtherBodyIndex :type Integer))
  (if (Variables|Default|GetbMovedObject?)
    (Utilities|FlowControl|DoOnce false
      (:Completed
        _)))
  (Utilities|Casting|CastToBP_ThirdPersonCharacterCustom OtherActor)
  (Widget|RemovefromParent (stale OnComponentBeginOverlap(Box) _returnvalue)))

(event EventBeginPlay)

(event Collision|EventActorBeginOverlap
  (params (OtherActor :type Actor%20Object%20Reference)))

(event EventTick
  (params (DeltaSeconds :type Float%20%28single-precision%29)))

(event EventInteract
  (bind _self self)
  (bind _defaultsceneroot (Variables|Default|GetDefaultSceneRoot _self))
  (bind _returnvalue (Transformation|GetWorldLocation _defaultsceneroot))
  (Utilities|FlowControl|DoOnce false
    (:Completed
      (Audio|PlaySound2D "/Engine/VREditor/Sounds/VR_grab.VR_grab" 1.0 1.0 0.0 0 0)
      (bind _newtrack_0 (Timeline|Timeline Play)
        (:Update
          (Transformation|SetActorRelativeLocation (Math|Vector|Lerp(Vector) _returnvalue (- _returnvalue "2.000000,0.000000,0.000000") _newtrack_0))
          (Variables|Default|SetbMovedObject? true))))))

(fn ConstructionScript)